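; Base enemy character that hurts the VR player on contact and explodes.
; A capsule overlap with a VRPawn calls its GettingHit, then a once-only explode event spawns Explosion_BP and destroys the enemy.
; Separate events turn on mesh physics for ragdolling and destroy the actor after a despawn delay.
; BeginPlay applies the configurable walk speed, and a controller UnPossess call is left unconnected.
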(event OnComponentBeginOverlap(CapsuleComponent)
  (params (OverlappedComponent :type Primitive%20Component%20Object%20Reference) (OtherActor :type Actor%20Object%20Reference) (OtherComp :type Primitive%20Component%20Object%20Reference) (OtherBodyIndex :type Integer) (bFromSweep :type Boolean) (SweepResult :type Hit%20Result%20Structure%20%28by%20ref%29))
  (bind _asvrpawn (Utilities|Casting|CastToVRPawn OtherActor))
  (Default|GettingHit _asvrpawn)
  (CallFunction|Explode))

(event Custom|BeginDespawn
  (Utilities|FlowControl|Delay (Variables|Default|GetDespawn_Timer))
  (Actor|DestroyActor))

(event Custom|RagdollEvent
  (Physics|SetSimulatePhysics (Variables|Character|GetMesh) true))

(event Custom|explode
  (Utilities|FlowControl|DoOnce false
    (:Completed
      (Game|SpawnActorfromClass "/Game/AI/explosion_BP.explosion_BP_C" (Transformation|GetActorTransform) "Undefined" "MultiplyWithRoot" 0 0)
      (Actor|DestroyActor))))

(event EventBeginPlay
  (Variables|/Script/Engine.CharacterMovementComponent|SetMaxWalkSpeed (Variables|Character|GetCharacterMovement) (Variables|Default|GetMax_Walk_Speed)))

(fn ConstructionScript)