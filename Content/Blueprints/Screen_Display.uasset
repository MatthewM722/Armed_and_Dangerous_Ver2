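; Screen_Display is an in-game display that shows the current wave and the kill count through two text elements.
; Custom events write supplied values straight into the wave and kill text.
; IncrementKillDisplay instead raises its own TotalKills counter and rebuilds the labeled kill text, while UpdateKills overwrites that text without changing the counter.
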(event Custom|Update%20Wave%20Display
  (params (Wave%20To%20Display :type Text))
  ;[1 1 1] Waves
  (Rendering|Components|TextRender|SetText (Variables|Default|GetWave_Display) Wave%20To%20Display))

(event Custom|Increment%20Kill%20Display
  ;[1 1 1] Kills
  (bind _result (Math|Integer|IncrementInt (Variables|Default|GetTotal_Kills))
    (:%20%20
      (Rendering|Components|TextRender|SetText (Variables|Default|GetKill_Display) (Utilities|Text|ToText(String) (Utilities|String|Append "Total Kills: " (Utilities|String|ToString(Integer) _result)))))))

(event Custom|Update%20Kills
  (params (CurrentKills_Input :type Text))
  (Rendering|Components|TextRender|SetText (Variables|Default|GetKill_Display) CurrentKills_Input))

(fn ConstructionScript)