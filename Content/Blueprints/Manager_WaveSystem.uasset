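; Wave manager that runs two timed enemy waves, starting shortly after BeginPlay.
; CurrentWave selects a Timeline whose event track spawns base enemies; its finish increments the wave and re-enters the switch after WaveDelay.
; Each wave start updates the wave display on all screens in TotalScreens.
; Spawning picks a random SpawnPoints entry, though the random range's upper bound is the array length, one past the last index.
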(event Custom|Begin%20Wave%20System
  (Utilities|FlowControl|Delay 5.0)
  (switch int (Variables|Default|GetCurrent_Wave)
    (:1
      ;[1 1 1] Wave 1
      (for _array_element (Variables|Default|GetTotal%20Screens)
        (Default|UpdateWaveDisplay _array_element "Wave 1"))
      (Timeline|Wave_1 Play
        (:Finished
          (Math|Integer|IncrementInt (Variables|Default|GetCurrent_Wave)
            (:%20%20
              (CallFunction|NewWave))))
        (:Enemy_Type_1
          (Utilities|SpawnEnemy "/Game/Enemy_AI/BP_Enemy_Base.BP_Enemy_Base_C"))))
    (:2
      ;[1 1 1] Wave 2
      (for _array_element_2 (Variables|Default|GetTotal%20Screens)
        (Default|UpdateWaveDisplay _array_element_2 "Wave 2"))
      (Timeline|Timeline Play
        (:Finished
          (Math|Integer|IncrementInt (Variables|Default|GetCurrent_Wave)
            (:%20%20
              (CallFunction|NewWave))))
        (:Enemy_Type_1
          (Utilities|SpawnEnemy "/Game/Enemy_AI/BP_Enemy_Base.BP_Enemy_Base_C"))))))

(event Custom|New%20Wave
  (Utilities|FlowControl|Delay (Variables|Default|GetWave_Delay))
  (switch int (Variables|Default|GetCurrent_Wave)
    (:1
      ;[1 1 1] Wave 1
      (for _array_element (Variables|Default|GetTotal%20Screens)
        (Default|UpdateWaveDisplay _array_element "Wave 1"))
      (Timeline|Wave_1 Play
        (:Finished
          (Math|Integer|IncrementInt (Variables|Default|GetCurrent_Wave)
            (:%20%20
              (CallFunction|NewWave))))
        (:Enemy_Type_1
          (Utilities|SpawnEnemy "/Game/Enemy_AI/BP_Enemy_Base.BP_Enemy_Base_C"))))
    (:2
      ;[1 1 1] Wave 2
      (for _array_element_2 (Variables|Default|GetTotal%20Screens)
        (Default|UpdateWaveDisplay _array_element_2 "Wave 2"))
      (Timeline|Timeline Play
        (:Finished
          (Math|Integer|IncrementInt (Variables|Default|GetCurrent_Wave)
            (:%20%20
              (CallFunction|NewWave))))
        (:Enemy_Type_1
          (Utilities|SpawnEnemy "/Game/Enemy_AI/BP_Enemy_Base.BP_Enemy_Base_C"))))))

(event EventBeginPlay
  (CallFunction|BeginWaveSystem))

(fn ConstructionScript)