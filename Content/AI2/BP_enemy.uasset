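; Enemy AI Blueprint that chases the VR player once its PawnSensing component spots them.
; Seeing any pawn sets a seeing flag and calls FollowPlayer, which moves it toward the VR pawn's camera position projected onto the navmesh, stopping within an acceptance radius.
; A separate RagdollEvent turns on physics simulation for the mesh.
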(event OnSeePawn(PawnSensing)
  (params (Pawn :type Pawn%20Object%20Reference))
  (Variables|Default|SetisSeeingPlayer true)
  (CallFunction|FollowPlayer))

(event Custom|FollowPlayer
  (if (Variables|Default|GetisSeeingPlayer)
    (bind _asvrpawn (Utilities|Casting|CastToVRPawn (Game|Player|GetPlayerPawn 0)))
    (AI|AIMoveTo self (.ProjectedLocation (AI|Navigation|ProjectPointtoNavigation (Transformation|GetWorldLocation (Variables|/Game/Blueprints/VRPawn.VRPawn_C|GetCamera _asvrpawn)) 0 0 "0, 0, 0")) 0 2.5e+02 false)))

(event Custom|RagdollEvent
  (Physics|SetSimulatePhysics (Variables|Character|GetMesh) true))

(fn ConstructionScript)